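; BP_TriggerTuto is a tutorial trigger volume that reacts when the player character overlaps its Box.
; The Tuto value selects the response: show one of two tutorial widgets for a few seconds, or open the Menu level after the same delay.
; RemoveWidget fades a widget out through a Delay-based loop that lowers render opacity, then removes it from its parent.
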(event OnComponentBeginOverlap(Box)
  (params (OverlappedComponent :type Primitive%20Component%20Object%20Reference) (OtherActor :type Actor%20Object%20Reference) (OtherComp :type Primitive%20Component%20Object%20Reference) (OtherBodyIndex :type Integer) (bFromSweep :type Boolean) (SweepResult :type Hit%20Result%20Structure%20%28by%20ref%29))
  (if (== OtherActor (Game|GetPlayerCharacter 0))
    (switch int (Variables|Default|GetTuto)
      (:1
        (bind _returnvalue (UserInterface|CreateWidget "/Game/Blueprints/HUD/WDG_TutoUI_1.WDG_TutoUI_1_C"))
        (UserInterface|Viewport|AddtoViewport _returnvalue 0)
        (Utilities|FlowControl|Delay 5.0)
        (CallFunction|RemoveWidget _returnvalue))
      (:2
        (bind _returnvalue_2 (UserInterface|CreateWidget "/Game/Blueprints/HUD/WDG_TutoUI_2.WDG_TutoUI_2_C"))
        (UserInterface|Viewport|AddtoViewport _returnvalue_2 0)
        (Utilities|FlowControl|Delay 5.0)
        (CallFunction|RemoveWidget _returnvalue_2))
      (:3
        (Utilities|FlowControl|Delay 5.0)
        (Game|OpenLevel(byName) "Menu")))))

(event Custom|Remove%20Widget
  (params (Widget :type Widget%20Object%20Reference))
  (bind _returnvalue (Class|Widget|GetRenderOpacity Widget))
  (if (> _returnvalue 0.0) :!label _label
    (Widget|SetRenderOpacity Widget (- _returnvalue 0.1))
    (Utilities|FlowControl|Delay 0.02)
    (goto _label)
    (else
      (Widget|RemovefromParent Widget))))

(event EventBeginPlay)

(event Collision|EventActorBeginOverlap
  (params (OtherActor :type Actor%20Object%20Reference)))

(event EventTick
  (params (DeltaSeconds :type Float%20%28single-precision%29)))

(fn ConstructionScript)