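; Default pawn Blueprint that lets the player grab and release things through a GrabberTP reference.
; Pressing the Grab input action calls Grab on GrabberTP, and releasing it calls Release.
; Helper functions return the actor's name and location, but the debug prints that use them are disconnected, and the other events are empty.
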(event EventBeginPlay)

(event Collision|EventActorBeginOverlap
  (params (OtherActor :type Actor%20Object%20Reference)))

(event EventTick
  (params (DeltaSeconds :type Float%20%28single-precision%29)))

(event Input|ActionEvents|InputActionGrab
  (params (Key :type Key%20Structure :default "None"))
  (bind _grabbertp (Variables|Default|GetGrabberTP))
  (:Pressed
    (Class|GrabberTP|Grab _grabbertp))
  (:Released
    (Class|GrabberTP|Release _grabbertp)))

(fn ConstructionScript)

(fn GetName
  (return (Utilities|GetObjectName self)))

(fn GetLocation
  (return (Transformation|GetActorLocation self)))