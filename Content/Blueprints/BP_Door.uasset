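; Door actor that swings open and closed on request from its OpenDoorTP member.
; OpenDoorRequest plays the Open timeline, which scales its track by OpenAngle to set the Door's relative yaw, and CloseDoorRequest reverses it.
; An older TriggerZone check summing overlapping mass against a threshold is disconnected, and the OpenDoor and CloseDoor events it calls are empty.
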(event OpenDoorRequest(OpenDoorTP)
  (bind _newtrack_0 (Timeline|Open Play)
    (:Update
      (Transformation|SetRelativeRotation (Variables|Default|GetDoor) (Math|Rotator|MakeRotator 0.0 0.0 (* _newtrack_0 (Variables|Default|GetOpenAngle))) false false))))

(event CloseDoorRequest(OpenDoorTP)
  (bind _newtrack_0 (Timeline|Open Reverse)
    (:Update
      (Transformation|SetRelativeRotation (Variables|Default|GetDoor) (Math|Rotator|MakeRotator 0.0 0.0 (* _newtrack_0 (Variables|Default|GetOpenAngle))) false false))))

(event Custom|OpenDoor)

(event Custom|CloseDoor)

(event EventBeginPlay)

(event Collision|EventActorBeginOverlap
  (params (OtherActor :type Actor%20Object%20Reference)))

(event EventTick
  (params (DeltaSeconds :type Float%20%28single-precision%29)))

(fn ConstructionScript)